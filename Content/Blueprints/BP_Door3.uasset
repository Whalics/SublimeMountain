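; Interactable swinging door that rotates 90 degrees open or closed in a direction set by the player's side.
; Interact stores the Player, updates DoorState and uses a FlipFlop to play or reverse a yaw Timeline, ignoring input while animating.
; DirectionTrigger overlaps track whether that stored Player is inside, which picks the swing sign on opening.
; Both overlap events also print the current direction for debugging.
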(event `/Game/Blueprints/BPI_Interactable.Interact`
  (params (Player :type "/Game/FirstPerson/Blueprints/BP_FirstPersonCharacter Object Reference"))
  (set `self.Player` Player)
  (if (not (`self.Animating`))
    (set `self.Animating` true)
    (switch `/Game/Blueprints/EDoorState` (`self.Door State`)
      (:`NewEnumerator0`
        (set `self.Door State` "NewEnumerator3"))
      (:`NewEnumerator1`
        (set `self.Door State` "NewEnumerator2")
        (set `self.TempDirection` (`KismetMathLibrary.SelectFloat` -90.0 90.0 (`self.In`)))))
    (`/Engine/EditorBlueprintResources/StandardMacros.FlipFlop`
      (:`A`
        (bind (_direction _alpha) (`Timeline|Timeline` :!via `PlayFromStart` :!label _label)
          (:`Update`
            (`SceneComponent.K2_SetRelativeRotation` (`self.Door`) (`KismetMathLibrary.MakeRotator` 0.0 0.0 (`KismetMathLibrary.Lerp` 0.0 (`self.TempDirection`) _alpha)) false false))
          (:`Finished`
            (set `self.Animating` false)
            (switch `/Game/Blueprints/EDoorState` (`self.Door State`)
              (:`NewEnumerator2`
                (set `self.Door State` "NewEnumerator0"))
              (:`NewEnumerator3`
                (set `self.Door State` "NewEnumerator1"))))))
      (:`B`
        (goto _label :!via `ReverseFromEnd`)))))

(event `self.Direction Trigger.OnComponentBeginOverlap`
  (params (OverlappedComponent :type "PrimitiveComponent Object Reference") (OtherActor :type "Actor Object Reference") (OtherComp :type "PrimitiveComponent Object Reference") (OtherBodyIndex :type Integer) (bFromSweep :type Boolean) (SweepResult :type "HitResult Structure (by ref)"))
  (if (== OtherActor (`self.Player`))
    (set `self.In` true)
    (`KismetSystemLibrary.PrintString` (`KismetStringLibrary.Conv_DoubleToString` (`self.TempDirection`)) :!label _label_2)))

(event `self.Direction Trigger.OnComponentEndOverlap`
  (params (OverlappedComponent :type "PrimitiveComponent Object Reference") (OtherActor :type "Actor Object Reference") (OtherComp :type "PrimitiveComponent Object Reference") (OtherBodyIndex :type Integer))
  (if (== OtherActor (`self.Player`))
    (set `self.In` false)
    (goto _label_2)))

(fn `UserConstructionScript`
  (`parent.UserConstructionScript`))