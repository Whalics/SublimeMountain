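; BP_Font is an interactable mana font that refills the player's mana to maximum.
; Its Interact event adds the difference between the player's max and current mana, then creates a screen flash widget on the viewport.
; If SingleUse is set, it also swaps the item mesh to an invisible material and plays a 2D sound, without destroying the actor.
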(event `/Game/Blueprints/BPI_Interactable.Interact`
  (params (Player :type "/Game/FirstPerson/Blueprints/BP_FirstPersonCharacter Object Reference"))
  (`/Game/FirstPerson/Blueprints/BP_FirstPersonCharacter.IncreaseMana` Player (- (`/Game/DataAssets/PDA_General.Max Mana` (`/Game/FirstPerson/Blueprints/BP_FirstPersonCharacter.GeneralData` Player)) (`/Game/FirstPerson/Blueprints/BP_FirstPersonCharacter.CurrMana` Player)))
  (bind _returnvalue (`|CreateWidget` "/Game/UI/WBP_ScreenFlash.WBP_ScreenFlash_C"))
  (`UserWidget.AddToViewport` _returnvalue 0)
  (if (`self.SingleUse`)
    (`PrimitiveComponent.SetMaterial` (`self.ItemMesh`) 0 "/Game/Art/MI_Invisible.MI_Invisible")
    (`GameplayStatics.PlaySound2D` (`self.SandQ`) 1.0 1.0 0.0 null null)))

(fn `UserConstructionScript`
  (`parent.UserConstructionScript`))