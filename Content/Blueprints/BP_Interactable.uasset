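; Base interactable item actor with a mesh, optional physics and a selectable trigger volume.
; Begin runs from both the construction script and BeginPlay, applying the mass override and physics setting, then enabling query-only collision on the chosen box, capsule or sphere trigger and hiding all three.
; GetPrompt exposes the input action, action text and item name, and ReturnSingleUsed reports single-use state.
; Interact and ChildInteract are empty here.
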(event `self.ReceiveBeginPlay`
  (`self.begin`))

(event `/Game/Blueprints/BPI_Interactable.Interact`
  (params (Player :type "/Game/FirstPerson/Blueprints/BP_FirstPersonCharacter Object Reference")))

(fn `begin`
  (bind _sphere_trigger (`self.Sphere Trigger`))
  (bind _itemmesh (`self.ItemMesh`))
  (bind _capsule_trigger (`self.Capsule Trigger`))
  (bind _sphere_trigger_2 (`self.Sphere Trigger`))
  (bind _sphere_trigger_3 (`self.Sphere Trigger`))
  (bind _box_trigger (`self.Box Trigger`))
  (bind _box_trigger_2 (`self.Box Trigger`))
  (bind _box_trigger_3 (`self.Box Trigger`))
  (bind _capsule_trigger_2 (`self.Capsule Trigger`))
  (bind _capsule_trigger_3 (`self.Capsule Trigger`))
  (`PrimitiveComponent.SetMassOverrideInKg` _itemmesh "None" (`self.Mass`) true)
  (if (`self.hasPhysics`)
    (`PrimitiveComponent.SetSimulatePhysics` _itemmesh true)
    (else
      (`PrimitiveComponent.SetSimulatePhysics` _itemmesh false)))
  (switch `/Game/E_TriggerType` (`self.ETriggerType`)
    (:`NewEnumerator0`
      (`SceneComponent.SetVisibility` _box_trigger false false)
      (`PrimitiveComponent.SetCollisionEnabled` _box_trigger "QueryOnly")
      (`SceneComponent.SetVisibility` _sphere_trigger_3 false false)
      (`PrimitiveComponent.SetCollisionEnabled` _sphere_trigger_3 "NoCollision")
      (`SceneComponent.SetVisibility` _capsule_trigger_2 false false)
      (`PrimitiveComponent.SetCollisionEnabled` _capsule_trigger_2 "NoCollision"))
    (:`NewEnumerator1`
      (`SceneComponent.SetVisibility` _capsule_trigger_3 false false)
      (`PrimitiveComponent.SetCollisionEnabled` _capsule_trigger_3 "QueryOnly")
      (`SceneComponent.SetVisibility` _sphere_trigger false false)
      (`PrimitiveComponent.SetCollisionEnabled` _sphere_trigger "NoCollision")
      (`SceneComponent.SetVisibility` _box_trigger_2 false false)
      (`PrimitiveComponent.SetCollisionEnabled` _box_trigger_2 "NoCollision"))
    (:`NewEnumerator2`
      (`SceneComponent.SetVisibility` _sphere_trigger_2 false false)
      (`PrimitiveComponent.SetCollisionEnabled` _sphere_trigger_2 "QueryOnly")
      (`SceneComponent.SetVisibility` _box_trigger_3 false false)
      (`PrimitiveComponent.SetCollisionEnabled` _box_trigger_3 "NoCollision")
      (`SceneComponent.SetVisibility` _capsule_trigger false false)
      (`PrimitiveComponent.SetCollisionEnabled` _capsule_trigger "NoCollision"))))

(fn `ChildInteract`)

(fn `GetPrompt`
  (returns (InputAction :type "InputAction Object Reference") (ActionText :type Text) (ItemName :type Text))
  (return (`self.Input Action`) (`self.Action Text`) (`self.Item Name`)))

(fn `ReturnSingleUsed`
  (returns (`Single Use` :type Boolean) (Used :type Boolean))
  (return (`self.SingleUse`) (`self.Used`)))

(fn `UserConstructionScript`
  (`self.begin`))