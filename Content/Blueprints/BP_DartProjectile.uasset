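; BP_DartProjectile is a short-lived dart that damages what it strikes.
; On capsule overlap it sends a fixed DamagedMessage to actors implementing BPI_Damage and destroys itself; it also destroys itself on other overlaps, with a check intended to spare BP_FirstPersonCharacter.
; A BeginPlay delay destroys darts after a few seconds.
; The Shard hit event is empty, and some leftover debug nodes are disconnected.
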(event `self.Shard.OnComponentHit`
  (params (HitComponent :type "PrimitiveComponent Object Reference") (OtherActor :type "Actor Object Reference") (OtherComp :type "PrimitiveComponent Object Reference") (NormalImpulse :type "Vector Structure") (Hit :type "HitResult Structure (by ref)")))

(event `self.ReceiveBeginPlay`
  (`KismetSystemLibrary.Delay` 5.0)
  (`self.K2_DestroyActor`))

(event `self.Capsule.OnComponentBeginOverlap`
  (params (OverlappedComponent :type "PrimitiveComponent Object Reference") (OtherActor :type "Actor Object Reference") (OtherComp :type "PrimitiveComponent Object Reference") (OtherBodyIndex :type Integer) (bFromSweep :type Boolean) (SweepResult :type "HitResult Structure (by ref)"))
  (if (`KismetSystemLibrary.DoesImplementInterface` OtherActor "/Game/Blueprints/Target/BPI_Damage.BPI_Damage_C")
    (message `/Game/Blueprints/Target/BPI_Damage.Damaged` OtherActor 5)
    (`self.K2_DestroyActor`)
    (elif (!= OtherActor "/Game/FirstPerson/Blueprints/BP_FirstPersonCharacter.BP_FirstPersonCharacter")
      (`self.K2_DestroyActor`))))

(fn `UserConstructionScript`)