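; BP_Button2 is an interactable button actor that resets the target system's score and the player's vials.
; Interact plays a press sound and runs the Animate timeline at a raised play rate, driving the button mesh's Z scale between zero and full.
; When the timeline finishes, it calls ResetScore on TargetSystem, then casts the player character to BP_FirstPersonCharacter and calls ResetVials.
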(event `/Game/Blueprints/BPI_Interactable.Interact`
  (params (Player :type "/Game/FirstPerson/Blueprints/BP_FirstPersonCharacter Object Reference"))
  (`GameplayStatics.PlaySoundAtLocation` "/Game/Audio/ButtonPress.ButtonPress" (`SceneComponent.RelativeLocation` (`self.DefaultSceneRoot`)) (struct) 1.0 1.0 0.0 null null null null)
  (`TimelineComponent.SetPlayRate` (`self.Animate`) 6.0)
  (bind (_direction _alpha) (`Timeline|Animate` :!via `PlayFromStart`)
    (:`Update`
      (`SceneComponent.SetWorldScale3D` (`self.SM_Button`) (`KismetMathLibrary.MakeVector` 1.0 1.0 (`KismetMathLibrary.Lerp` 0.0 1.0 _alpha))))
    (:`Finished`
      (`/Game/Blueprints/Target/BP_TargetSpawner.Reset Score` (`self.TargetSystem`))
      (bind _asbp_first_person_character (cast `/Game/FirstPerson/Blueprints/BP_FirstPersonCharacter` (`GameplayStatics.GetPlayerCharacter` 0)))
      (`/Game/FirstPerson/Blueprints/BP_FirstPersonCharacter.ResetVials` _asbp_first_person_character))))

(fn `UserConstructionScript`
  (`parent.UserConstructionScript`))