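; Elevator actor that raises its platform to an upper stop when any actor overlaps it.
; On overlap it stores the platform's world Z as the lower stop, then plays the DoorAnimation timeline after a one-second retriggerable delay.
; The timeline lerps the platform's relative Z from that world-space value to UpperStop's relative Z, keeping X and Y.
; No descent logic is present.
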(event `self.ReceiveActorBeginOverlap`
  (params (OtherActor :type "Actor Object Reference"))
  (bind _elevator_platform (`self.Elevator Platform`))
  (bind _returnvalue (`SceneComponent.GetRelativeTransform` (`self.Elevator Platform`)))
  (bind (_returnvalue_x _returnvalue_y _returnvalue_z) (`KismetMathLibrary.BreakVector` (`SceneComponent.K2_GetComponentLocation` _elevator_platform)))
  (bind (_relativelocation_x _relativelocation_y _relativelocation_z) (`KismetMathLibrary.BreakVector` (`SceneComponent.RelativeLocation` (`self.UpperStop`))))
  ;[1 1 1] Door Animation
  (set `self.Lower Stop` _returnvalue_z)
  (`KismetSystemLibrary.RetriggerableDelay` 1.0)
  (bind (_direction _moveplatform) (`Timeline|DoorAnimation`)
    (:`Update`
      (`SceneComponent.K2_SetRelativeLocation` _elevator_platform (`KismetMathLibrary.MakeVector` (.x (.location _returnvalue)) (.y (.location _returnvalue)) (`KismetMathLibrary.Lerp` (`self.Lower Stop`) _relativelocation_z _moveplatform)) false false))))

(fn `UserConstructionScript`)