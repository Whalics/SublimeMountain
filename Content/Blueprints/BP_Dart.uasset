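; BP_Dart is a dart Blueprint that plays a spawn effect on its Shard component when play begins.
; Flash creates a dynamic instance of M_Overlay, sets it as the Shard's overlay material, and drives its ES scalar parameter from the MaterialFlash timeline.
; In parallel, Scale uses the StartScale timeline to grow the Shard's world scale uniformly between zero and full size.
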(event `Flash`
  (bind _returnvalue (`KismetMaterialLibrary.CreateDynamicMaterialInstance` "/Game/Art/LevelPrototyping/Dart/M_Overlay.M_Overlay"))
  (bind _output_get (set `self.OverlayMat` _returnvalue))
  (`MeshComponent.SetOverlayMaterial` (`self.Shard`) _output_get)
  (bind (_direction _newtrack_0) (`Timeline|MaterialFlash` :!via `PlayFromStart`)
    (:`Update`
      (`MaterialInstanceDynamic.SetScalarParameterValue` (`self.OverlayMat`) "ES" _newtrack_0))))

(event `Scale`
  (bind (_direction _alpha) (`Timeline|StartScale` :!via `PlayFromStart`)
    (:`Update`
      (bind _returnvalue (`KismetMathLibrary.Lerp` 0.0 1.0 _alpha))
      (`SceneComponent.SetWorldScale3D` (`self.Shard`) (`KismetMathLibrary.MakeVector` _returnvalue _returnvalue _returnvalue)))))

(event `self.ReceiveBeginPlay`
  (`self.Flash`)
  (`self.Scale`))

(fn `UserConstructionScript`)