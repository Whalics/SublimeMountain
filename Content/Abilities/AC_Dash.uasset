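; Dash ability component for the player, with separate ground and air tuning loaded from data on BeginPlay.
; Setup computes start and end points and sets play rates on the player's timelines; UpdateDash lerps location with sweep, queuing jumps.
; Finishing sets velocity along the dash from clamped pre-dash momentum plus an upward boost.
; A retriggerable-delay cooldown gates reuse, with dashes restored on the ground or upon landing.
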(event `Landed`
  (if (not (`self.bDisable`))
    (`self.Reset Dash`)))

(event `self.ReceiveBeginPlay`
  (`parent.ReceiveBeginPlay`)
  (`self.SetDashData`))

(event `StartDashCooldown`
  ;[1 1 1] Dash Cooldown
  (set `self.bCanDash` false)
  (set `self.bCooldown` true)
  (`KismetSystemLibrary.RetriggerableDelay` (`self.Cooldown`))
  (set `self.bCooldown` false)
  (if (`self.isGrounded`)
    (`self.Reset Dash`)
    (`KismetSystemLibrary.PrintString` "Cooldown ended")))

(event `On Finished Dashing`
  (set `MovementComponent.Velocity` (`self.CalcPostDashVelocity`) (`self.Character Movement`))
  (if (not (`self.bCooldown`))
    (`self.EndDash`)))

(fn `EndDash`
  (set `self.bIsDashing` false)
  (set `self.bDisable` false)
  (if (`self.isGrounded`)
    (`self.Reset Dash`)))

(fn `Reset Dash`
  (if (not (`self.bCooldown`))
    (set `self.bCanDash` true)
    (set `self.DashCounter` 1)
    (set `self.Max Dashes` 0)))

(fn `SetDashData`
  (bind _data (`self.Data`))
  (`|ExecutionSequence`
    (:`then_0`
      (set `self.AirDistance` (`/Game/DataAssets/PDA_Dash.AirDistance` _data)))
    (:`then_1`
      (set `self.AirSpeed` (`/Game/DataAssets/PDA_Dash.AirSpeed` _data)))
    (:`then_2`
      (set `self.Cooldown` (`/Game/DataAssets/PDA_Dash.Cooldown` _data)))
    (:`then_3`
      (set `self.PostSpeedMin` (`/Game/DataAssets/PDA_Dash.Post Speed Minimum` _data)))
    (:`then_4`
      (set `self.ManaCost` (`/Game/DataAssets/PDA_Dash.Mana Cost` _data)))
    (:`then_5`
      (set `self.PostSpeedMax` (`/Game/DataAssets/PDA_Dash.Post Speed Minimum` _data)))
    (:`then_6`
      (set `self.AirUpBoost` (`/Game/DataAssets/PDA_Dash.AirUpBoost` _data)))
    (:`then_7`
      (set `self.GroundSpeed` (`/Game/DataAssets/PDA_Dash.GroundSpeed` _data)))
    (:`then_8`
      (set `self.GroundDistance` (`/Game/DataAssets/PDA_Dash.GroundDistance` _data)))
    (:`then_9`
      (set `self.GroundUpBoost` (`/Game/DataAssets/PDA_Dash.GroundUpBoost` _data)))))

(fn `SetupDash`
  (bind (_startpoint _endpoint) (`self.GetAirDashPoints` (`/Game/FirstPerson/Blueprints/BP_FirstPersonCharacter.GetDirection` (`self.Player`))))
  (bind (_startpoint_2 _endpoint_2) (`self.GetGroundDashPoints` (`/Game/FirstPerson/Blueprints/BP_FirstPersonCharacter.GetDirection` (`self.Player`))))
  (`self.StartDashCooldown`)
  (set `self.bIsDashing` true)
  (if (`self.isGrounded`)
    (set `self.StartPoint` _startpoint_2)
    (set `self.EndPoint` _endpoint_2)
    (else
      (set `self.StartPoint` _startpoint)
      (set `self.EndPoint` _endpoint)))
  (set `self.PreDashSpeed` (`self.CalcPreDashSpeed`))
  (`|ExecutionSequence`
    (:`then_0`
      (`TimelineComponent.SetPlayRate` (`/Game/FirstPerson/Blueprints/BP_FirstPersonCharacter.GroundDashTimeline` (`self.Player`)) (`self.GroundSpeed`)))
    (:`then_1`
      (`TimelineComponent.SetPlayRate` (`/Game/FirstPerson/Blueprints/BP_FirstPersonCharacter.AirDashTimeline` (`self.Player`)) (`self.AirSpeed`)))))

(fn `Try To Dash`
  (returns (`Started Dashing` :type Boolean))
  (if (`self.bCanDash`)
    (`/Game/FirstPerson/Blueprints/BP_FirstPersonCharacter.Dash` (`self.Player`))
    (`KismetSystemLibrary.PrintString` "Tried to dash")
    (return true)
    (else
      (return false))))

(fn `UpdateDash`
  (params (Alpha :type "Float (double-precision)"))
  (returns (StopDash :type Boolean))
  (if (`self.bDisable`)
    (return true)
    (else
      (bind (_sweephitresult _returnvalue) (`Actor.K2_SetActorLocation` (`self.Player`) (`KismetMathLibrary.VLerp` (`self.StartPoint`) (`self.EndPoint`) (`local.Alpha`)) true false))
      (if _returnvalue
        (if (`Character.bPressedJump` (`self.Player`))
          (set `self.bQueueJump` true))
        (return false)
        (else
          (return true))))))