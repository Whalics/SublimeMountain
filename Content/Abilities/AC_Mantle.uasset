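; Player ability component that automatically mantles the character onto ledges, with a Tick-driven state machine for checking, mantling and cooldown.
; Detection rejects nearby ground or ceiling, then chains capsule and wall traces to validate the ledge and choose quick or regular mantle.
; Movement uses Flying mode with input ignored, interpolating view and swept vertical and horizontal position toward the goal.
; It returns to Falling on timeout or a vertical trace hit.
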(event `self.ReceiveTick`
  (params (DeltaSeconds :type "Float (single-precision)"))
  (switch `/Game/Blueprints/E_MantleState` (`self.MantleState`)
    (:`NewEnumerator0`
      (bind (_mantlestate _height) (`self.CheckCanMantle`))
      (bind _output_get (set `self.MantleState` _mantlestate))
      (switch `/Game/Blueprints/E_MantleState` _output_get
        (:`NewEnumerator1`
          _)
        (:`NewEnumerator4`
          _))
      (`self.SetupMantle` _height))
    (:`NewEnumerator1`
      (bind _completed (`self.MantleMovement` DeltaSeconds :!label _label))
      (if _completed
        (`self.EndMantle`)
        (set `self.MantleState` "NewEnumerator2")
        (`KismetSystemLibrary.Delay` (`/Game/DataAssets/PDA_Mantle.Cooldown` (`self.Data`)))
        (set `self.MantleState` "NewEnumerator0")))
    (:`NewEnumerator4`
      (goto _label))))

(fn `CheckCanMantle`
  (returns (MantleState :type "/Game/Blueprints/E_MantleState Enum") (Height :type "Float (double-precision)"))
  (if (`self.MantleChecks`)
    (bind (_outhit _returnvalue) (`self.LineTraceUpAndDown`))
    (if _returnvalue
      (return "NewEnumerator0" 0.0)
      (else
        (bind (_outhit_2 _returnvalue_2) (`self.DoMantleLineTrace` (`Actor.GetActorForwardVector` (`self.Player`))))
        (if _returnvalue_2
          (bind _outhit_3 (`self.DoWallLineTrace` (.z (`.Location` (`GameplayStatics.BreakHitResult` _outhit_2)))))
          (bind (_returnvalue_3 _direction _speedtowardswall) (`self.CheckWallHit` _outhit_3))
          (if _returnvalue_3
            (bind _output_get (set `self.DirectionTowardsWall` _direction))
            (bind _outhit_4 (`self.DoMantleLineTrace` _output_get))
            (if (`self.CheckHitForMantle` _outhit_4)
              (set `self.GoalPosition` (`self.GetGoalPosition` _outhit_4))
              (bind (_mantle_state _height) (`self.CheckForQuickMantle` _outhit_4))
              (return _mantle_state _height)
              (else
                (return "NewEnumerator0" 0.0)))
            (else
              (return "NewEnumerator0" 0.0)))
          (else
            (return "NewEnumerator0" 0.0)))))
    (else
      (return "NewEnumerator0" 0.0))))

(fn `DoMantleLineTrace`
  (params (Direction :type "Vector Structure"))
  (returns (OutHit :type "HitResult Structure") (ReturnValue :type Boolean))
  (bind (_eyes _feet) (`self.MantleVectors`))
  (bind _returnvalue (* Direction (`/Game/DataAssets/PDA_Mantle.MaxDistanceAwayFromWall` (`self.Data`))))
  (bind (_outhit _returnvalue_2) (`KismetSystemLibrary.CapsuleTraceSingleForObjects` :`Start` (+ _eyes _returnvalue) :`End` (+ _feet _returnvalue) :`Radius` 20.0 :`HalfHeight` 10.0 :`ObjectTypes` (`|MakeArray` "ObjectTypeQuery1" :!type "EObjectTypeQuery Enum") :`DrawDebugType` (`self.DrawDebugType`)))
  (return _outhit _returnvalue_2))

(fn `DoWallLineTrace`
  (params (Z :type "Float (double-precision)"))
  (returns (OutHit :type "HitResult Structure"))
  (bind (_returnvalue_x _returnvalue_y) (`KismetMathLibrary.BreakVector` (`Actor.K2_GetActorLocation` (`self.Player`))))
  (bind _returnvalue (`KismetMathLibrary.MakeVector` _returnvalue_x _returnvalue_y (- Z (`/Game/DataAssets/PDA_Mantle.MinLedgeHeight` (`self.Data`)))))
  (bind _outhit (`KismetSystemLibrary.LineTraceSingleForObjects` :`Start` _returnvalue :`End` (+ _returnvalue (* (`Actor.GetActorForwardVector` (`self.Player`)) (`/Game/DataAssets/PDA_Mantle.MaxDistanceAwayFromWall` (`self.Data`)) 2.0)) :`ObjectTypes` (`|MakeArray` "ObjectTypeQuery1" :!type "EObjectTypeQuery Enum") :`DrawDebugType` (`self.DrawDebugType`)))
  (return _outhit))

(fn `EndMantle`
  (`CharacterMovementComponent.SetMovementMode` (`self.Character Movement`) "MOVE_Falling" 0)
  (`Controller.SetIgnoreMoveInput` (`Pawn.GetController` (`self.Player`)) false))

(fn `LineTraceUpAndDown`
  (returns (OutHit :type "HitResult Structure") (ReturnValue :type Boolean))
  (bind (_outhit _returnvalue) (`self.VerticalLineTrace` false))
  (if _returnvalue
    (return _outhit _returnvalue)
    (else
      (bind (_outhit_2 _returnvalue_2) (`self.VerticalLineTrace` true))
      (return _outhit_2 _returnvalue_2))))

(fn `MantleMovement`
  (params (`Delta Time` :type "Float (double-precision)"))
  (returns (Completed :type Boolean))
  (bind (_goalposition_x _goalposition_y _goalposition_z) (`KismetMathLibrary.BreakVector` (`self.GoalPosition`)))
  (bind (_goalposition_x_2 _goalposition_y_2) (`KismetMathLibrary.BreakVector` (`self.GoalPosition`)))
  (bind _returnvalue (`Pawn.GetController` (`self.Player`)))
  (bind (_returnvalue_x _returnvalue_y _returnvalue_z) (`KismetMathLibrary.BreakVector` (`Actor.K2_GetActorLocation` (`self.Player`))))
  (bind _looklerpusesz (`/Game/DataAssets/PDA_Mantle.LookLerpUsesZ` (`self.Data`)))
  (`Controller.SetControlRotation` _returnvalue (`KismetMathLibrary.RInterpTo` (`Controller.GetControlRotation` _returnvalue) (`KismetMathLibrary.FindLookAtRotation` (`KismetMathLibrary.MakeVector` _returnvalue_x _returnvalue_y (`KismetMathLibrary.SelectFloat` _returnvalue_z 0.0 _looklerpusesz)) (`KismetMathLibrary.MakeVector` _goalposition_x_2 _goalposition_y_2 (`KismetMathLibrary.SelectFloat` _goalposition_z 0.0 _looklerpusesz))) (`GameplayStatics.GetWorldDeltaSeconds`) (`/Game/DataAssets/PDA_Mantle.LookSpeed` (`self.Data`))))
  (`Actor.K2_SetActorLocation` (`self.Player`) (`self.GetVerticalPos`) true false)
  (`Actor.K2_SetActorLocation` (`self.Player`) (`self.GetHorizontalPos`) true false)
  (bind _output_get (set `self.TimePassed` (+ (`self.TimePassed`) (`local.Delta Time`))))
  (if (>= _output_get (`/Game/DataAssets/PDA_Mantle.MaxTimeAllowed` (`self.Data`)))
    (return true)
    (else
      (bind (_outhit _returnvalue_2) (`self.LineTraceUpAndDown`))
      (return _returnvalue_2))))

(fn `SetupMantle`
  (params (Height :type "Float (double-precision)"))
  (bind (_returnvalue_roll _returnvalue_pitch) (`KismetMathLibrary.BreakRotator` (`Pawn.GetControlRotation` (`self.Player`))))
  (`self.StartedMantle` Height _returnvalue_pitch)
  (`CharacterMovementComponent.SetMovementMode` (`self.Character Movement`) "MOVE_Flying" 0)
  (set `MovementComponent.Velocity` (0.0 0.0 0.0) (`self.Character Movement`))
  (`Controller.SetIgnoreMoveInput` (`Pawn.GetController` (`self.Player`)) true)
  (set `self.TimePassed` 0.0))

(fn `TryToMantle`)

(fn `VerticalLineTrace`
  (params (Up :type Boolean))
  (returns (OutHit :type "HitResult Structure") (ReturnValue :type Boolean))
  (locals (NewLocalVar :type "Array of EObjectTypeQuery Enum"))
  (bind _returnvalue (`Actor.K2_GetActorLocation` (`self.Player`)))
  (bind (_outhit _returnvalue_2) (`KismetSystemLibrary.LineTraceSingleForObjects` _returnvalue (+ (* (`KismetMathLibrary.SelectVector` (0.0 0.0 1.0) (0.0 0.0 -1.0) Up) (+ (`CapsuleComponent.GetScaledCapsuleHalfHeight` (`Character.CapsuleComponent` (`self.Player`))) (`/Game/DataAssets/PDA_Mantle.GroundCheckDistance` (`self.Data`)))) _returnvalue) (`|MakeArray` "ObjectTypeQuery1" :!type "EObjectTypeQuery Enum")))
  (return _outhit _returnvalue_2))