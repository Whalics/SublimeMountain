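; Assault rifle weapon Blueprint that traces shots from its muzzle and notifies damageable actors.
; WeaponTrace runs a camera trace to find the aim point, then sphere-traces on Visibility from the Muzzle toward it, drawing both traces for debugging.
; A hit actor implementing BPI_Damage receives a Damaged message with no parameters.
; The event graph holds only disabled stubs, and nothing in this Blueprint calls WeaponTrace.
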(fn `UserConstructionScript`
  (`parent.UserConstructionScript`))

(fn `WeaponTrace`
  (bind _returnvalue (`SceneComponent.K2_GetComponentLocation` (`self.Muzzle`)))
  (bind _outhit (`/Game/Blueprints/Libraries/BPFL_Traces.CameraTrace` 5000.0 1.0 "ForDuration"))
  (bind _outhit_2 (`KismetSystemLibrary.SphereTraceSingle` :`Start` _returnvalue :`End` (+ _returnvalue (* (`KismetMathLibrary.GetForwardVector` (`KismetMathLibrary.FindLookAtRotation` _returnvalue (`.ImpactPoint` (`GameplayStatics.BreakHitResult` _outhit)))) 8000.0)) :`Radius` 1.0 :`TraceChannel` "TraceTypeQuery1" :`DrawDebugType` "ForDuration"))
  (if (`KismetSystemLibrary.DoesImplementInterface` (`.HitActor` (`GameplayStatics.BreakHitResult` _outhit_2)) "/Game/Blueprints/Target/BPI_Damage.BPI_Damage_C")
    (message `/Game/Blueprints/Target/BPI_Damage.Damaged` (`.HitActor` (`GameplayStatics.BreakHitResult` _outhit_2)))))