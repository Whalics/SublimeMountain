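; Dart ability component that lets the player prime, aim and fire a dart projectile at a mana cost, with optional camera zoom.
; Prime spawns a preview dart, which Tick lerps toward the weapon spawn point and rotates toward the camera trace target.
; FireProjectile launches a separate projectile using the unsmoothed aim rotation, destroys the preview, then ends zoom and spends mana if primed.
; DestroyDart cancels a primed dart without firing.
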(event `self.ReceiveTick`
  (params (DeltaSeconds :type "Float (single-precision)"))
  (`/Engine/EditorBlueprintResources/StandardMacros.IsValid` (`self.DartInstance`)
    (:`Is Valid`
      (`self.Set Dart Transform`))))

(fn `DestroyDart`
  (`/Engine/EditorBlueprintResources/StandardMacros.IsValid` (`self.DartInstance`)
    (:`Is Valid`
      (`Actor.K2_DestroyActor` (`self.DartInstance`))
      (set `self.DartInstance` null)
      (`self.Primed?`
        (:`true`
          (`/Game/FirstPerson/Blueprints/BP_FirstPersonCharacter.End Zoom Camera` (`self.Player`))
          (set `self.bPrimed` false))))))

(fn `FireProjectile`
  (bind _player (`self.Player`))
  (`/Engine/EditorBlueprintResources/StandardMacros.IsValid` (`self.DartInstance`)
    (:`Is Valid`
      (if (`self.CanFire`)
        (`KismetSystemLibrary.PrintString` "Fired")
        (`/Game/FirstPerson/Blueprints/BP_FirstPersonCharacter.PlayCameraShake` (`self.Player`) "/Game/CameraShake/FireProjectile.FireProjectile_C")
        (bind (_lerprotation _realrotation) (`self.Set Projectile Rotation`))
        (`|SpawnActorFromClass` "/Game/Blueprints/BP_DartProjectile.BP_DartProjectile_C" (`KismetMathLibrary.MakeTransform` (`self.Get Spawn Location`) _realrotation) "Undefined" "MultiplyWithRoot" null null)
        (`GameplayStatics.PlaySound2D` (`self.FireQ`) 1.0 1.0 0.0 null null)
        (`Actor.K2_DestroyActor` (`self.DartInstance`))
        (set `self.DartInstance` null)
        (`self.Primed?`
          (:`true`
            (`/Game/FirstPerson/Blueprints/BP_FirstPersonCharacter.End Zoom Camera` _player)
            (`/Game/FirstPerson/Blueprints/BP_FirstPersonCharacter.DecrementMana` _player (`/Game/DataAssets/PDA_Dart.Mana Cost` (`self.Data`)))))))))

(fn `Get Spawn Location`
  (returns (ReturnValue :type "Vector Structure"))
  (return (`SceneComponent.K2_GetComponentLocation` (`/Game/FirstPerson/Blueprints/BP_FirstPersonCharacter.WeaponSpawnPoint` (`self.Player`)))))

(fn `HoldZoom`
  (params (`Hold Time` :type "Float (double-precision)") (Playrate :type "Float (double-precision)" :default 1.5))
  (if (`self.CanFire`)
    (if (> `Hold Time` (`/Game/DataAssets/PDA_Dart.ZoomTime` (`self.Data`)))
      (`/Game/FirstPerson/Blueprints/BP_FirstPersonCharacter.Zoom Camera` (`self.Player`) Playrate))))

(fn `LerpToPosition`
  (returns (ReturnValue :type "Vector Structure"))
  (return (`KismetMathLibrary.VLerp` (`Actor.K2_GetActorLocation` (`self.DartInstance`)) (`SceneComponent.K2_GetComponentLocation` (`/Game/FirstPerson/Blueprints/BP_FirstPersonCharacter.WeaponSpawnPoint` (`self.Player`))) (`/Game/DataAssets/PDA_Dart.FollowLerpAlpha` (`self.Data`)))))

(fn `Prime`
  (returns (Output_Get :type "/Game/Blueprints/BP_Dart Object Reference"))
  (`/Engine/EditorBlueprintResources/StandardMacros.IsValid` (`self.DartInstance`)
    (:`Is Not Valid`
      (if (`self.CanFire`)
        (set `self.bPrimed` true)
        (bind _returnvalue (`|SpawnActorFromClass` (`self.Dart`) (`SceneComponent.K2_GetComponentToWorld` (`/Game/FirstPerson/Blueprints/BP_FirstPersonCharacter.WeaponSpawnPoint` (`self.Player`))) "AlwaysSpawn" "MultiplyWithRoot" null null))
        (bind _output_get (set `self.DartInstance` _returnvalue))
        (`GameplayStatics.PlaySound2D` (`self.SpawnQ`) 1.0 1.0 0.0 null null)
        (return _output_get)))))

(fn `Set Dart Transform`
  (`/Engine/EditorBlueprintResources/StandardMacros.IsValid` (`self.DartInstance`)
    (:`Is Valid`
      (bind _lerprotation (`self.Set Projectile Rotation`))
      (bind _returnvalue (`self.LerpToPosition`))
      (`Actor.K2_SetActorLocationAndRotation` (`self.DartInstance`) _returnvalue _lerprotation false false))))

(fn `Set Projectile Rotation`
  (returns (LerpRotation :type "Rotator Structure") (RealRotation :type "Rotator Structure"))
  (bind _dartinstance (`self.DartInstance`))
  (bind (_out _bhit) (`/Game/FirstPerson/Blueprints/BP_FirstPersonCharacter.GetLineTraceFromCamera` (`self.Player`) 5000.0 "TraceTypeQuery1"))
  (bind (_bblockinghit _binitialoverlap _time _distance _location _impactpoint _normal _impactnormal _physmat _hitactor _hitcomponent _hitbonename _bonename _hititem _elementindex _faceindex _tracestart _traceend) (`GameplayStatics.BreakHitResult` _out))
  (bind (_returnvalue_roll _returnvalue_pitch _returnvalue_yaw) (`KismetMathLibrary.BreakRotator` (`KismetMathLibrary.FindLookAtRotation` (`Actor.K2_GetActorLocation` _dartinstance) (`KismetMathLibrary.SelectVector` _impactpoint _traceend _bhit))))
  (bind _returnvalue (`KismetMathLibrary.MakeRotator` _returnvalue_roll (+ _returnvalue_pitch 0.0) _returnvalue_yaw))
  (return (`KismetMathLibrary.RLerp` (`SceneComponent.K2_GetComponentRotation` (`/Game/Blueprints/BP_Dart.Shard` _dartinstance)) _returnvalue (`/Game/DataAssets/PDA_Dart.RotateLerpAlpha` (`self.Data`)) true) _returnvalue))

(fn `TriggerPrime`
  (`self.HoldZoom` 1.0 2.0)
  (`self.Prime`)
  (set `self.bCanFireFromBurrow` false))